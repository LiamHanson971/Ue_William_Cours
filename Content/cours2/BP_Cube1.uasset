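; BP_Cube1 is an actor that spins around its yaw axis while bobbing up and down.
; Each Tick it adds a fixed local yaw rotation and shifts its Z location by Speed, without sweep or delta-time scaling.
; Speed flips sign when Z exactly equals AmplitudeTop or AmplitudeBotton, so the reversal depends on the steps landing precisely on those limits.
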(event EventBeginPlay)

(event Collision|EventActorBeginOverlap
  (params (OtherActor :type Actor%20Object%20Reference)))

(event EventTick
  (params (DeltaSeconds :type Float%20%28single-precision%29))
  (bind _self self)
  (bind _returnvalue (Transformation|GetActorTransform _self))
  (bind _location (Math|Transform|BreakTransform _returnvalue))
  (bind (_x _y _z) (Math|Vector|BreakVector _location))
  (Transformation|AddActorLocalRotation (Math|Rotator|MakeRotator 0.0 0.0 3.0) false false)
  (Variables|Default|SetHeigh (Math|Vector|MakeVector _x _y (+ _z (Variables|Default|GetSpeed))))
  (Transformation|SetActorLocation (Variables|Default|GetHeigh) false false)
  (if (== (.Z (Math|Vector|BreakVector (.Location (Math|Transform|BreakTransform (Transformation|GetActorTransform self))))) (Variables|Default|GetAmplitudeTop))
    (Variables|Default|SetSpeed -1)
    (elif (== (.Z (Math|Vector|BreakVector (.Location (Math|Transform|BreakTransform (Transformation|GetActorTransform self))))) (Variables|Default|GetAmplitudeBotton))
      (Variables|Default|SetSpeed 1))))

(fn ConstructionScript)