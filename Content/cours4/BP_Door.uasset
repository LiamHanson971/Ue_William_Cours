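; BP_Door is a door actor that lowers its Cube component when a BP_ThirdPersonCharacter enters its Box trigger.
; The overlap moves the Cube to a sunken relative location via MoveComponentTo; leaving the trigger only prints a debug message.
; Separate OpenDoor and CloseDoor functions look unfinished and are not called here: one steps actor height by Speed, the other applies a zero rotation.
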(event OnComponentBeginOverlap(Box)
  (params (OverlappedComponent :type Primitive%20Component%20Object%20Reference) (OtherActor :type Actor%20Object%20Reference) (OtherComp :type Primitive%20Component%20Object%20Reference) (OtherBodyIndex :type Integer) (bFromSweep :type Boolean) (SweepResult :type Hit%20Result%20Structure%20%28by%20ref%29))
  (Utilities|Casting|CastToBP_ThirdPersonCharacter OtherActor)
  (Development|PrintString "col")
  (Components|MoveComponentTo (Variables|Default|GetCube) "0.000000,0.000000,-150.000000" "0, 0, 0" false false 0.2 false))

(event OnComponentEndOverlap(Box)
  (params (OverlappedComponent :type Primitive%20Component%20Object%20Reference) (OtherActor :type Actor%20Object%20Reference) (OtherComp :type Primitive%20Component%20Object%20Reference) (OtherBodyIndex :type Integer))
  (Utilities|Casting|CastToBP_ThirdPersonCharacter OtherActor)
  (Development|PrintString "end col"))

(event Custom|Open%20Door)

(event EventBeginPlay)

(event Collision|EventActorBeginOverlap
  (params (OtherActor :type Actor%20Object%20Reference)))

(event EventTick
  (params (DeltaSeconds :type Float%20%28single-precision%29)))

(fn ConstructionScript)

(fn OpenDoor
  (bind _self self)
  (bind _returnvalue (Transformation|GetActorTransform _self))
  (bind _location (Math|Transform|BreakTransform _returnvalue))
  (bind (_x _y _z) (Math|Vector|BreakVector _location))
  (Variables|Default|SetHeigh (Math|Vector|MakeVector _x _y (+ _z (Variables|Default|GetSpeed))))
  (Transformation|SetActorLocation (Variables|Default|GetHeigh) false false)
  (if (== (.Z (Math|Vector|BreakVector (.Location (Math|Transform|BreakTransform (Transformation|GetActorTransform self))))) (Variables|Default|GetAmplitudeTop))
    (Variables|Default|SetSpeed -1)
    (elif true
      (Variables|Default|SetSpeed 0))))

(fn CloseDoor
  (Transformation|AddActorLocalRotation "0.000000,0.000000,0.000000" false false))